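; BP_Puzzle1_Manager manages a button-order puzzle that guards a door.
; RegisterButtonPress appends the pressed index to PlayerSequence and compares that newest entry with the same position in CorrectSequence, but nothing follows the comparison.
; A separate PuzzleSuccess event destroys DoorToDelete and is not called within this graph.
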(event Custom|PuzzleSuccess
  (Actor|DestroyActor (Variables|Default|GetDoorToDelete)))

(event Custom|RegisterButtonPress
  (params (PressedIndex :type Integer))
  (bind _playersequence (Variables|Default|GetPlayerSequence))
  (bind _returnvalue (Utilities|Array|LastIndex _playersequence))
  (Utilities|Array|Add (Variables|Default|GetPlayerSequence) PressedIndex)
  (if (== (Utilities|Array|Get(acopy) (Variables|Default|GetPlayerSequence) _returnvalue) (Utilities|Array|Get(acopy) (Variables|Default|GetCorrectSequence) _returnvalue))
    _))

(fn ConstructionScript)