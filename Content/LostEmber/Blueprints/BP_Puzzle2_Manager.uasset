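; BP_Puzzle2_Manager is a puzzle manager that opens the way past a door once three plates are active at once.
; Every Tick it checks the IsActive flag on Plate1, Plate2 and Plate3.
; When all three are true, it destroys the DoorToDelete actor, with no guard against repeating the call on later frames.
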(event EventTick
  (params (DeltaSeconds :type Float%20%28single-precision%29))
  (if (and (and (Variables|/Game/LostEmber/Blueprints/BP_PP.BP_PP_C|GetIsActive (Variables|Default|GetPlate1)) (Variables|/Game/LostEmber/Blueprints/BP_PP.BP_PP_C|GetIsActive (Variables|Default|GetPlate2))) (Variables|/Game/LostEmber/Blueprints/BP_PP.BP_PP_C|GetIsActive (Variables|Default|GetPlate3)))
    (Actor|DestroyActor (Variables|Default|GetDoorToDelete))))

(fn ConstructionScript)