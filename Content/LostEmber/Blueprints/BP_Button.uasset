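; BP_Button is an interactive button actor that tracks whether the player orb is in range and whether it is activated.
; InteractionZone overlaps with BP_PlayerOrb toggle PlayerInRange.
; ActivateButton only sets IsActivated, while ResetButton clears it and restores the M_Button material.
; BeginPlay enables player input, though no input events are handled here, and leftover dynamic-material colour and CurrentButton-clearing nodes are disconnected.
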(event OnComponentBeginOverlap(InteractionZone)
  (params (OverlappedComponent :type Primitive%20Component%20Object%20Reference) (OtherActor :type Actor%20Object%20Reference) (OtherComp :type Primitive%20Component%20Object%20Reference) (OtherBodyIndex :type Integer) (bFromSweep :type Boolean) (SweepResult :type Hit%20Result%20Structure%20%28by%20ref%29))
  (bind _asbp_player_orb (Utilities|Casting|CastToBP_PlayerOrb OtherActor))
  (Variables|Default|SetbPlayerInRange true))

(event OnComponentEndOverlap(InteractionZone)
  (params (OverlappedComponent :type Primitive%20Component%20Object%20Reference) (OtherActor :type Actor%20Object%20Reference) (OtherComp :type Primitive%20Component%20Object%20Reference) (OtherBodyIndex :type Integer))
  (Utilities|Casting|CastToBP_PlayerOrb OtherActor)
  (Variables|Default|SetbPlayerInRange false))

(event Custom|ActivateButton
  (Variables|Default|SetIsActivated true))

(event Custom|ResetButton
  (Variables|Default|SetIsActivated false)
  (Rendering|Material|SetMaterial (Variables|Default|GetButtonMesh) 0 "/Game/LostEmber/Blueprints/M_Button.M_Button"))

(event Collision|EventActorBeginOverlap
  (params (OtherActor :type Actor%20Object%20Reference)))

(event EventTick
  (params (DeltaSeconds :type Float%20%28single-precision%29)))

(event EventBeginPlay
  (Input|EnableInput (Game|GetPlayerController 0)))

(fn ConstructionScript)