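; BP_PP is a pressure-plate style trigger that turns on while the player or a box enters its interaction zone.
; Begin and end overlap on InteractionZone check for the Player or Box actor tag, set the IsActive flag and print a debug message.
; It keeps no overlap count, so any tagged actor leaving clears IsActive even if another remains inside.
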(event OnComponentBeginOverlap(InteractionZone)
  (params (OverlappedComponent :type Primitive%20Component%20Object%20Reference) (OtherActor :type Actor%20Object%20Reference) (OtherComp :type Primitive%20Component%20Object%20Reference) (OtherBodyIndex :type Integer) (bFromSweep :type Boolean) (SweepResult :type Hit%20Result%20Structure%20%28by%20ref%29))
  (if (or (Actor|ActorHasTag OtherActor "Player") (Actor|ActorHasTag OtherActor "Box"))
    (Variables|Default|SetIsActive true)
    (Development|PrintString "PP activated")))

(event OnComponentEndOverlap(InteractionZone)
  (params (OverlappedComponent :type Primitive%20Component%20Object%20Reference) (OtherActor :type Actor%20Object%20Reference) (OtherComp :type Primitive%20Component%20Object%20Reference) (OtherBodyIndex :type Integer))
  (if (or (Actor|ActorHasTag OtherActor "Player") (Actor|ActorHasTag OtherActor "Box"))
    (Variables|Default|SetIsActive false)
    (Development|PrintString "PP desactivated")))

(fn ConstructionScript)