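; BP_PlayerOrb is the player-controlled glowing orb in LostEmber.
; Axis inputs add movement relative to control yaw and turn the view through controller yaw and pitch.
; The Interact input activates CurrentButton after a validity check; this graph never assigns that reference.
; A timeline started at BeginPlay drives both the point light intensity and the glow effect's PulseAlpha parameter from one scaled pulse value.
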(event EventBeginPlay
  (bind _pulsevalue (Timeline|TL_LightPulse Play)
    (:Update
      (Niagara|SetNiagaraVariable(Float) (Variables|Default|GetOrbGlowFX) "User.PulseAlpha" (* _pulsevalue 1.5e+03))
      (Rendering|Components|Light|SetIntensity (Variables|Default|GetPointLight) (* _pulsevalue 1.5e+03)))))

(event Collision|EventActorBeginOverlap
  (params (OtherActor :type Actor%20Object%20Reference)))

(event EventTick
  (params (DeltaSeconds :type Float%20%28single-precision%29)))

(event Input|ActionEvents|InputActionInteract
  (params (Key :type Key%20Structure :default "None"))
  (:Pressed
    (Utilities|IsValid 0
      (:Is%20Valid
        (Default|ActivateButton (Variables|Default|GetCurrentButton))))))

(event Input|AxisEvents|InputAxisMoveForward
  (params (AxisValue :type Float%20%28single-precision%29))
  (Pawn|Input|AddMovementInput (Math|Vector|GetForwardVector (Math|Rotator|MakeRotator 0.0 0.0 (.Yaw (Math|Rotator|BreakRotator (Pawn|GetControlRotation :!class /Script/Engine.Pawn))))) AxisValue false))

(event Input|AxisEvents|InputAxisMoveRight
  (params (AxisValue :type Float%20%28single-precision%29))
  (Pawn|Input|AddMovementInput (Math|Vector|GetRightVector (Math|Rotator|MakeRotator 0.0 0.0 (.Yaw (Math|Rotator|BreakRotator (Pawn|GetControlRotation :!class /Script/Engine.Pawn))))) AxisValue false))

(event Input|AxisEvents|InputAxisTurn
  (params (AxisValue :type Float%20%28single-precision%29))
  (Pawn|Input|AddControllerYawInput AxisValue))

(event Input|AxisEvents|InputAxisLookUP
  (params (AxisValue :type Float%20%28single-precision%29))
  (Pawn|Input|AddControllerPitchInput AxisValue))

(fn ConstructionScript)